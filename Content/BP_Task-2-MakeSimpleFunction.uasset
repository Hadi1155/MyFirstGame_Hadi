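; A practice actor Blueprint for making a simple function: it keeps a Score and prints it as debug text.
; BeginPlay prints the starting Score.
; Tick runs through a one-second Delay, which throttles calls to MenambahkanScoreBy10s to roughly once per second.
; That function adds 10 to Score and prints the new total; overlap and construction logic are empty.
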(event EventBeginPlay
  (Development|PrintString (Utilities|String|Append "My Score is : " (Utilities|String|ToString(Integer) (Variables|Default|GetScore)))))

(event Collision|EventActorBeginOverlap
  (params (OtherActor :type Actor%20Object%20Reference)))

(event EventTick
  (params (DeltaSeconds :type Float%20%28single-precision%29))
  (Utilities|FlowControl|Delay 1.0)
  (CallFunction|MenambahkanScoreBy=10/s))

(fn ConstructionScript)

(fn MenambahkanScoreBy=10/s
  (bind _output_get (Variables|Default|SetScore (+ (Variables|Default|GetScore) 10)))
  (Development|PrintString (Utilities|String|Append "Now My Score is : " (Utilities|String|ToString(Integer) _output_get))))