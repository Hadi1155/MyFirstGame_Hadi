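; Base enemy Blueprint that patrols, chases and shoots the player's BP_Eva, and ragdolls briefly before being destroyed at zero HP.
; Patrol loops AI moves to random nearby reachable points.
; Pawn sensing triggers a chase that turns to the target and fires a muzzle line trace applying damage, with effects and sound.
; A retriggerable delay resumes patrol once sightings stop; the shoot montage node is disconnected.
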(event OnSeePawn(PawnSensing)
  (params (Pawn :type Pawn%20Object%20Reference))
  (bind _asbp_eva (Utilities|Casting|CastToBP_Eva Pawn))
  (CallFunction|ChasePlayer _asbp_eva)
  (Utilities|FlowControl|RetriggerableDelay 1.0)
  (CallFunction|Patrol))

(event Custom|Patrol
  (Variables|/Script/Engine.CharacterMovementComponent|SetMaxWalkSpeed (Variables|Character|GetCharacterMovement) (Variables|Default|GetPatrolSpeed))
  (AI|AIMoveTo self (.RandomLocation (AI|Navigation|GetRandomReachablePointinRadius (Transformation|GetActorLocation) 4e+02 0 0)) 0 5.0 false
    (:OnSuccess
      (Utilities|FlowControl|Delay 0.01)
      (CallFunction|Patrol))))

(event Custom|Attack
  (params (Character :type BP%20Eva%20Object%20Reference))
  (bind _armed (Variables|Default|GetArmed))
  (bind _returnvalue (Transformation|GetSocketLocation _armed "Muzzle"))
  (Transformation|SetActorRotation (Math|Rotator|FindRelativeLookatRotation (Math|Conversions|ToTransform(Vector) (Transformation|GetActorLocation)) (Transformation|GetActorLocation Character)))
  (Effects|SpawnEmitterAttached "/Game/Realistic_Starter_VFX_Pack_Vol2/Particles/Explosion/P_Explosion_Big_A.P_Explosion_Big_A" _armed "Muzzle" "0, 0, 0" "0, 0, 0" "0.100000,0.100000,0.100000")
  (Audio|PlaySoundatLocation "/Game/Focus/Assets/Audios/Weapon-SFX/AR4_SFX.AR4_SFX" "0, 0, 0" "0, 0, 0" 1.0 1.0 0.0 0 0 0 0)
  (bind _outhit (Collision|LineTraceByChannel _returnvalue (+ _returnvalue (* (Math|Random|RandomUnitVectorinConeinDegrees (Math|Vector|GetForwardVector (Transformation|GetActorRotation)) 0.0) 2e+03)) "TraceTypeQuery1" false 0 "ForDuration" true "(R=0.844924,G=1.000000,B=0.000000,A=1.000000)" "(R=0.000000,G=1.000000,B=0.000000,A=1.000000)" 0.05))
  (Game|Damage|ApplyDamage (.HitActor (Collision|BreakHitResult _outhit)) 5.0 0 0))

(event Custom|ChasePlayer
  (params (TargetActor :type BP%20Eva%20Object%20Reference))
  (Variables|/Script/Engine.CharacterMovementComponent|SetMaxWalkSpeed (Variables|Character|GetCharacterMovement) (Variables|Default|GetChaseSpeed))
  (AI|AIMoveTo self "0, 0, 0" TargetActor (Variables|Default|GetAcceptance%20Radius) false
    (:then
      _)
    (:OnSuccess
      _)
    (:OnFail
      _))
  (Transformation|SetActorRotation (Math|Rotator|FindRelativeLookatRotation (Math|Conversions|ToTransform(Vector) (Transformation|GetActorLocation)) (Transformation|GetActorLocation TargetActor)))
  (CallFunction|Attack TargetActor))

(event EventBeginPlay
  (CallFunction|Patrol))

(event Game|Damage|EventAnyDamage
  (params (Damage :type Float%20%28single-precision%29) (DamageType :type Damage%20Type%20Object%20Reference) (InstigatedBy :type Controller%20Object%20Reference) (DamageCauser :type Actor%20Object%20Reference))
  (Audio|PlaySoundatLocation "/Game/Focus/Assets/Audios/BaseSFX/SC_HitSFX.SC_HitSFX" "0, 0, 0" "0, 0, 0" 1.0 1.0 0.0 0 0 0 0)
  (if (not (Variables|Default|GetIsDead))
    (bind _output_get (Variables|Default|SetCurrentHP (- (Variables|Default|GetCurrentHP) Damage)))
    (Development|PrintString (Utilities|String|ToString(Float) _output_get))
    (if (<= (Variables|Default|GetCurrentHP) 0.0)
      (Variables|Default|SetIsDead true)
      (Audio|PlaySoundatLocation "/Game/Focus/Assets/Audios/Enemies-SFX/SC_GunnerDeath.SC_GunnerDeath" "0, 0, 0" "0, 0, 0" 1.0 1.0 0.0 0 0 0 0)
      (Physics|SetSimulatePhysics (Variables|Character|GetMesh) true)
      (Utilities|FlowControl|Delay 1.0)
      (Actor|DestroyActor))))

(fn ConstructionScript)