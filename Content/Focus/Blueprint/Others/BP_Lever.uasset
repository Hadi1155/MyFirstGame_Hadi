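; BP_Lever is an interactable lever that, when used, marks itself activated and broadcasts an OnLeverActivated event.
; OnInteract also spawns an explosion effect, plays two sounds and runs a timeline that flips the handle 180 degrees on roll.
; It caches a BP_HugeDoor reference on BeginPlay and exposes its state through GetLeverStatus.
; It always reports itself interactable, so it can be retriggered, and its detection text is empty.
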(event EventBeginPlay
  (bind _returnvalue (Actor|GetActorOfClass "/Game/Focus/Blueprint/Others/BP_HugeDoor.BP_HugeDoor_C"))
  (bind _asbp_huge_door (Utilities|Casting|CastToBP_HugeDoor _returnvalue))
  (Variables|Default|SetDoorRef _asbp_huge_door))

(event Collision|EventActorBeginOverlap
  (params (OtherActor :type Actor%20Object%20Reference)))

(event EventTick
  (params (DeltaSeconds :type Float%20%28single-precision%29)))

(event EventOnInteract
  (params (Character :type BP%20Eva%20Object%20Reference))
  (Variables|Default|SetIsActivated true)
  (Default|CallOnLeverActivated)
  (Effects|SpawnEmitteratLocation "/Game/Realistic_Starter_VFX_Pack_Vol2/Particles/Explosion/P_Explosion_Big_B.P_Explosion_Big_B" (Transformation|GetWorldLocation (Variables|Default|GetDefaultSceneRoot)))
  (Audio|PlaySoundatLocation "/Game/Focus/Assets/Audios/Interactables/Lever.Lever" "0, 0, 0" "0, 0, 0" 1.0 1.0 0.0 0 0 0 0)
  (Audio|PlaySoundatLocation "/Game/Focus/Assets/Audios/Interactables/Electro.Electro" "0, 0, 0" "0, 0, 0" 1.0 1.0 0.0 0 0 0 0)
  (bind _newtrack_0 (Timeline|Timeline PlayFromStart)
    (:Update
      (Transformation|SetRelativeRotation (Variables|Default|GetHandle) (Math|Rotator|MakeRotator (Math|Float|Lerp 0.0 1.8e+02 _newtrack_0) 0.0 0.0) false false))))

(fn ConstructionScript)

(fn GetLeverStatus
  (return (Variables|Default|GetIsActivated)))

(fn IsInteractable?
  (params (Character :type BP%20Eva%20Object%20Reference))
  (return true))

(fn OnDetected
  (return ""))