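; BP_HeartDrops is a collectible heart pickup that restores health to the character who picks it up.
; On pickup it passes HPToAdd to the character's AddHPNotice, then runs the parent pickup logic.
; CanBePickedUp calls the parent but decides only on HP, refusing pickup when CurrentHP equals MaxHP.
; An older inline heal that clamps to MaxHP remains in the event graph, disconnected.
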(event EventOnPickUp
  (params (Character :type BP%20Eva%20Object%20Reference))
  (Default|AddHPNotice Character (Variables|Default|GetHPToAdd))
  (|CallParentFunction 0))

(fn ConstructionScript
  (|CallParentFunction))

(fn CanbePickedUp?
  (params (Character :type BP%20Eva%20Object%20Reference))
  (|CallParentFunction Character)
  (if (== (Variables|/Game/Focus/Blueprint/Character/BP_Eva.BP_Eva_C|GetMaxHP Character) (Variables|/Game/Focus/Blueprint/Character/BP_Eva.BP_Eva_C|GetCurrentHP Character))
    (return false)
    (else
      (return true))))