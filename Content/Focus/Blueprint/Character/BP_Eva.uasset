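; BP_Eva is a player character with Enhanced Input walk, run and look controls and a single weapon slot.
; An overlap detector tracks a nearby BP_Weapon; pickup stores its weapon data, destroys the actor and shows the mesh on the back, dropping any held weapon first.
; Holster toggles the mesh between back and armed components, while drop spawns a new BP_Weapon in front from the stored data.
; The sprint input is unimplemented.
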(event OnComponentBeginOverlap(PickupDetector)
  (params (OverlappedComponent :type Primitive%20Component%20Object%20Reference) (OtherActor :type Actor%20Object%20Reference) (OtherComp :type Primitive%20Component%20Object%20Reference) (OtherBodyIndex :type Integer) (bFromSweep :type Boolean) (SweepResult :type Hit%20Result%20Structure%20%28by%20ref%29))
  (bind _asbp_weapon (Utilities|Casting|CastToBP_Weapon OtherActor))
  (Variables|Default|SetDetectedWeapon _asbp_weapon))

(event OnComponentEndOverlap(PickupDetector)
  (params (OverlappedComponent :type Primitive%20Component%20Object%20Reference) (OtherActor :type Actor%20Object%20Reference) (OtherComp :type Primitive%20Component%20Object%20Reference) (OtherBodyIndex :type Integer))
  (Variables|Default|SetDetectedWeapon 0))

(event Input|EnhancedActionEvents|EnhancedInputActionIA_Walk_Eva
  (params (ActionValue :type Vector%202D%20Structure) (ElapsedSeconds :type Float%20%28double-precision%29) (TriggeredSeconds :type Float%20%28double-precision%29) (InputAction :type Input%20Action%20Object%20Reference :default "/Game/Focus/Blueprint/Input_Eva/IA_Walk_Eva.IA_Walk_Eva"))
  (bind _returnvalue (Pawn|GetControlRotation :!class /Script/Engine.Pawn))
  (Pawn|Input|AddMovementInput (Math|Vector|GetRightVector (Pawn|GetControlRotation :!class /Script/Engine.Pawn)) (.x ActionValue) false)
  (Pawn|Input|AddMovementInput (Math|Vector|GetForwardVector (Math|Rotator|MakeRotator (.roll _returnvalue) 0.0 (.yaw _returnvalue))) (.y ActionValue) false))

(event Input|EnhancedActionEvents|EnhancedInputActionIA_Run_Eva
  (params (ActionValue :type Boolean) (ElapsedSeconds :type Float%20%28double-precision%29) (TriggeredSeconds :type Float%20%28double-precision%29) (InputAction :type Input%20Action%20Object%20Reference :default "/Game/Focus/Blueprint/Input_Eva/IA_Run_Eva.IA_Run_Eva"))
  (:Started
    (Variables|/Script/Engine.CharacterMovementComponent|SetMaxWalkSpeed (Variables|Character|GetCharacterMovement) (Variables|Default|GetRunSpeed)))
  (:Completed
    (Variables|/Script/Engine.CharacterMovementComponent|SetMaxWalkSpeed (Variables|Character|GetCharacterMovement) (Variables|Default|GetWalkingSpeed))))

(event Input|EnhancedActionEvents|EnhancedInputActionIA_Sprint_Eva
  (params (ActionValue :type Boolean) (ElapsedSeconds :type Float%20%28double-precision%29) (TriggeredSeconds :type Float%20%28double-precision%29) (InputAction :type Input%20Action%20Object%20Reference :default "/Game/Focus/Blueprint/Input_Eva/IA_Sprint_Eva.IA_Sprint_Eva")))

(event Input|EnhancedActionEvents|EnhancedInputActionIA_Look_Eva
  (params (ActionValue :type Vector%202D%20Structure) (ElapsedSeconds :type Float%20%28double-precision%29) (TriggeredSeconds :type Float%20%28double-precision%29) (InputAction :type Input%20Action%20Object%20Reference :default "/Game/Focus/Blueprint/Input_Eva/IA_Look_Eva.IA_Look_Eva"))
  (Pawn|Input|AddControllerYawInput (.x ActionValue))
  (Pawn|Input|AddControllerPitchInput (.y ActionValue)))

(event Input|EnhancedActionEvents|EnhancedInputActionIA_Pickup
  (params (ActionValue :type Boolean) (ElapsedSeconds :type Float%20%28double-precision%29) (TriggeredSeconds :type Float%20%28double-precision%29) (InputAction :type Input%20Action%20Object%20Reference :default "/Game/Focus/Blueprint/Input_Eva/IA_Pickup.IA_Pickup"))
  (:Started
    (Utilities|PickUpMacro)))

(event Input|EnhancedActionEvents|EnhancedInputActionIA_Drop_Eva
  (params (ActionValue :type Boolean) (ElapsedSeconds :type Float%20%28double-precision%29) (TriggeredSeconds :type Float%20%28double-precision%29) (InputAction :type Input%20Action%20Object%20Reference :default "/Game/Focus/Blueprint/Input_Eva/IA_Drop_Eva.IA_Drop_Eva"))
  (:Started
    (Utilities|DropWepMacro)))

(event Input|EnhancedActionEvents|EnhancedInputActionIA_Holster_Eva
  (params (ActionValue :type Boolean) (ElapsedSeconds :type Float%20%28double-precision%29) (TriggeredSeconds :type Float%20%28double-precision%29) (InputAction :type Input%20Action%20Object%20Reference :default "/Game/Focus/Blueprint/Input_Eva/IA_Holster_Eva.IA_Holster_Eva"))
  (:Started
    (Utilities|IsValid (Variables|Default|GetWeapon)
      (:Is%20Valid
        (if (Variables|Default|GetisWeaponHolstered?)
          (Variables|Default|SetisWeaponHolstered? false)
          (Components|SkeletalMesh|SetSkeletalMeshAsset (Variables|Default|GetArmed) (Variables|/Game/Focus/Blueprint/Weapons/WeaponDatas/BP_WeaponData.BP_WeaponData_C|GetWeaponMesh (Variables|Default|GetWeapon)))
          (Components|SkeletalMesh|SetSkeletalMeshAsset (Variables|Default|GetHolster%28%20Back%20%29) 0)
          (else
            (Variables|Default|SetisWeaponHolstered? true)
            (Components|SkeletalMesh|SetSkeletalMeshAsset (Variables|Default|GetArmed) 0)
            (Components|SkeletalMesh|SetSkeletalMeshAsset (Variables|Default|GetHolster%28%20Back%20%29) (Variables|/Game/Focus/Blueprint/Weapons/WeaponDatas/BP_WeaponData.BP_WeaponData_C|GetWeaponMesh (Variables|Default|GetWeapon)))))))))

(event EventBeginPlay
  (bind _asplayer_controller (Utilities|Casting|CastToPlayerController (Pawn|GetController)))
  (Input|AddMappingContext (PlayerController|LocalPlayerSubsystems|GetEnhancedInputLocalPlayerSubsystem _asplayer_controller) "/Game/Focus/Blueprint/Input_Eva/IMC_Eva.IMC_Eva" 0 "(bIgnoreAllPressedKeysUntilRelease=True,bForceImmediately=False,bNotifyUserSettings=False)")
  (Variables|/Script/Engine.CharacterMovementComponent|SetMaxWalkSpeed (Variables|Character|GetCharacterMovement) (Variables|Default|GetWalkingSpeed)))

(fn ConstructionScript)