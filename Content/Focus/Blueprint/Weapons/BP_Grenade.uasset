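; BP_Grenade is a grenade actor that explodes on a fixed fuse started at BeginPlay.
; The blast plays a sound and explosion emitter, then deals uniform radial damage, since the falloff radii and damage bounds match.
; It ignores itself, names the first player's character as damage causer, and destroys itself after a short delay.
; Its DamageOverlappedUnits function and construction script are empty.
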(event EventBeginPlay
  (Utilities|FlowControl|Delay 3.0)
  (Audio|PlaySoundatLocation "/Game/Focus/Assets/Audios/Weapon-SFX/080902_shotgun-39753.080902_shotgun-39753" (Transformation|GetActorLocation) "0, 0, 0" 1.0 1.0 0.0 0 0 0 0)
  (Effects|SpawnEmitteratLocation "/Game/Realistic_Starter_VFX_Pack_Vol2/Particles/Explosion/P_Explosion_Big_B.P_Explosion_Big_B" (Transformation|GetActorLocation) "0, 0, 0" "2.000000,2.000000,2.000000")
  (Class|GameplayStatics|ApplyRadialDamagewithFalloff 2e+02 2e+02 (Transformation|GetActorLocation) 1e+03 1e+03 0.0 0 (Utilities|Array|MakeArray self) (Game|GetPlayerCharacter 0) 0 "ECC_Visibility")
  (Utilities|FlowControl|Delay 2.0)
  (Actor|DestroyActor))

(fn ConstructionScript)

(fn DamageOverlappedUnits)