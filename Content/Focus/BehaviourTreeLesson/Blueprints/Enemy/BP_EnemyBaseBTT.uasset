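; Base enemy character for the behaviour tree lesson, providing melee attack, sword handling, patrol route and movement speed functions.
; Attack and sheathe play montages and call end dispatchers so callers know when they finish.
; Wielding spawns a BP_LS sword on the weapon socket, and a sheathe montage notify destroys it, with both updating the wielding flag.
; Getters expose the patrol route and fixed attack/defend ranges, while a speed enum sets max walk speed.
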(event Custom|Attack
  (Animation|Montage|PlayMontage (Variables|Character|GetMesh) "/Game/Focus/Blueprint/Enemy/Animations/MeleeAnim/AM_AlienSlash.AM_AlienSlash"
    (:OnCompleted
      _)
    (:OnInterrupted
      _))
  (Default|CallOnAttackEnd))

(event Custom|WieldLS
  (bind _returnvalue (Game|SpawnActorfromClass "/Game/Focus/BehaviourTreeLesson/MeleeWeapon/Blueprints/BP_LS.BP_LS_C" (Transformation|GetActorTransform) "Undefined" "MultiplyWithRoot" 0 0))
  (bind _output_get (Variables|Default|SetLS_Mesh _returnvalue))
  (Transformation|AttachComponentToComponent _output_get (Variables|Character|GetMesh) "WeaponSocket" "SnapToTarget" "SnapToTarget" "SnapToTarget" true)
  (Variables|Default|SetIsWieldingSword true))

(event Custom|SheatheSword
  (bind _notifyname (Animation|Montage|PlayMontage (Variables|Character|GetMesh) "/Game/Focus/BehaviourTreeLesson/Animations/Character/Mannequin-Only/AM_AlienSheathe.AM_AlienSheathe")
    (:OnCompleted
      (Default|CallOnSheatheEnd))
    (:OnNotifyBegin
      (switch name _notifyname
        (:DropWeapon
          (Actor|DestroyActor (Variables|Default|GetLS_Mesh))
          (Variables|Default|SetIsWieldingSword false))))))

(fn ConstructionScript)

(fn GetIdealRange
  (return 1.5e+02 3.5e+02))

(fn GetPatrolRoute
  (return (Variables|Default|GetPatrolRoute)))

(fn SetMovementSpeed
  (params (Speed :type E_AIMovementSpd%20Enum :default "NewEnumerator0"))
  (bind _output_get (Variables|/Script/Engine.CharacterMovementComponent|SetMaxWalkSpeed (Variables|Character|GetCharacterMovement) (Utilities|Select :Index Speed :NewEnumerator0 0.0 :NewEnumerator1 1e+02 :NewEnumerator2 3e+02 :NewEnumerator3 5e+02)))
  (return _output_get))