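; A destructible spawner nest that spawns small monsters in timed batches from BeginPlay.
; Each batch spawns a set number of BP_SmallMonsters at the nest's transform, adjusting for collisions, then a Delay loop repeats until the batch count runs out.
; Incoming damage lowers and prints the nest's HP, destroying the actor at zero.
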(event Custom|SpawnEnemy
  (params (DesiredEnemyCount :type Integer))
  (Variables|Default|SetSpawnEnemyCount DesiredEnemyCount)
  (while (> (Variables|Default|GetSpawnEnemyCount) 0)
    (Game|SpawnActorfromClass "/Game/Focus/Blueprint/Enemy/BP_SmallMonsters.BP_SmallMonsters_C" (Math|Transform|MakeTransform (Transformation|GetActorLocation) (Transformation|GetActorRotation) "1.000000,1.000000,1.000000") "AdjustIfPossibleButAlwaysSpawn" "MultiplyWithRoot" 0 0)
    (Variables|Default|SetSpawnEnemyCount (- (Variables|Default|GetSpawnEnemyCount) 1))))

(event Custom|BatchSpawnEnemy
  (params (BatchCount :type Integer) (EnemiesPerBatch :type Integer) (Interval :type Float%20%28double-precision%29))
  (Variables|Default|SetBatchCount BatchCount)
  (CallFunction|SpawnEnemy EnemiesPerBatch :!label _label)
  (Variables|Default|SetBatchCount (- (Variables|Default|GetBatchCount) 1))
  (Utilities|FlowControl|Delay Interval)
  (if (> (Variables|Default|GetBatchCount) 0)
    (goto _label)))

(event EventBeginPlay
  (CallFunction|BatchSpawnEnemy (Variables|Default|GetBatches) (Variables|Default|GetEnemies%20Per%20Batch) (Variables|Default|GetSpawnCooldownDur)))

(event Game|Damage|EventAnyDamage
  (params (Damage :type Float%20%28single-precision%29) (DamageType :type Damage%20Type%20Object%20Reference) (InstigatedBy :type Controller%20Object%20Reference) (DamageCauser :type Actor%20Object%20Reference))
  (if (not (Variables|Default|GetIsDead))
    (bind _output_get (Variables|Default|SetSpawnerNestHp (- (Variables|Default|GetSpawnerNestHp) Damage)))
    (Development|PrintString (Utilities|String|ToString(Float) _output_get))
    (if (<= (Variables|Default|GetSpawnerNestHp) 0.0)
      (Variables|Default|SetIsDead true)
      (Actor|DestroyActor))))

(fn ConstructionScript)