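; Melee enemy Blueprint from a behaviour tree lesson that handles taking damage and dying; its graphs contain no attack or AI logic.
; AnyDamage plays a hit sound on every hit, then, while alive, subtracts from CurrentHP and prints it.
; At zero HP it sets IsDead, plays a death sound, enables mesh physics and destroys the actor after a short delay.
; Both sounds play at the world origin rather than the enemy's position.
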(event EventBeginPlay)

(event Collision|EventActorBeginOverlap
  (params (OtherActor :type Actor%20Object%20Reference)))

(event EventTick
  (params (DeltaSeconds :type Float%20%28single-precision%29)))

(event Game|Damage|EventAnyDamage
  (params (Damage :type Float%20%28single-precision%29) (DamageType :type Damage%20Type%20Object%20Reference) (InstigatedBy :type Controller%20Object%20Reference) (DamageCauser :type Actor%20Object%20Reference))
  (Audio|PlaySoundatLocation "/Game/Focus/Assets/Audios/BaseSFX/SC_HitSFX.SC_HitSFX" "0, 0, 0" "0, 0, 0" 1.0 1.0 0.0 0 0 0 0)
  (if (not (Variables|Default|GetIsDead))
    (bind _output_get (Variables|Default|SetCurrentHP (- (Variables|Default|GetCurrentHP) Damage)))
    (Development|PrintString (Utilities|String|ToString(Float) _output_get))
    (if (<= (Variables|Default|GetCurrentHP) 0.0)
      (Variables|Default|SetIsDead true)
      (Audio|PlaySoundatLocation "/Game/Focus/Assets/Audios/Enemies-SFX/SC_GunnerDeath.SC_GunnerDeath" "0, 0, 0" "0, 0, 0" 1.0 1.0 0.0 0 0 0 0)
      (Physics|SetSimulatePhysics (Variables|Character|GetMesh) true)
      (Utilities|FlowControl|Delay 1.0)
      (Actor|DestroyActor))))

(fn ConstructionScript
  (|CallParentFunction))