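; BP_HugeDoor is a heavy door that opens upward once its required levers are activated.
; On BeginPlay it binds to the activation event of every BP_Lever in the level, and each activation rechecks its LeversToActivate list.
; If none is inactive and the count matches ValueToComplete, it calls HeavyDoorOpened, then after a short delay plays a sound and raises the mesh with a Timeline.
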(event Custom|CanDoorOpen?
  (if (== (Variables|Default|GetExecutedIndex) (Variables|Default|GetValueToComplete))
    (Default|CallHeavyDoorOpened)
    (Utilities|FlowControl|Delay 0.5)
    (CallFunction|OpenDoor)))

(event Custom|LeverCheck
  (Variables|Default|SetLoopBroke false)
  (Variables|Default|SetExecutedIndex 0)
  (bind _array_element (Utilities|Array|ForEachLoopwithBreak (Variables|Default|GetLeversToActivate) :!label _label)
    (:LoopBody
      (Utilities|IsValid _array_element
        (:Is%20Valid
          (if (Variables|/Game/Focus/Blueprint/Others/BP_Lever.BP_Lever_C|GetIsActivated _array_element)
            (Variables|Default|SetExecutedIndex (+ (Variables|Default|GetExecutedIndex) 1))
            (else
              (Variables|Default|SetLoopBroke true)
              (goto _label Break))))))
    (:Completed
      (if (not (Variables|Default|GetLoopBroke))
        (CallFunction|CanDoorOpen?)))))

(event Custom|OpenDoor
  (bind _returnvalue (Transformation|GetActorLocation))
  (Audio|PlaySoundatLocation "/Game/Focus/Assets/Audios/Interactables/HeavyDoor.HeavyDoor" "0, 0, 0" "0, 0, 0" 1.0 1.0 0.0 0 0 0 0)
  (bind _doornewlocation (Timeline|Timeline_0 PlayFromStart)
    (:Update
      (Transformation|SetWorldLocation (Variables|Default|GetMesh) (Math|Vector|MakeVector (.x _returnvalue) (.y _returnvalue) (+ (.z _returnvalue) (Math|Float|Lerp 0.0 6.0 _doornewlocation))) false false))))

(event EventBeginPlay
  (bind _outactors (Actor|GetAllActorsOfClass "/Game/Focus/Blueprint/Others/BP_Lever.BP_Lever_C"))
  (EventDispatchers|BindEventtoOnLeverActivated _outactors (delegate Custom|LeverCheck)))

(fn ConstructionScript)

(fn CheckIsLoopBroken
  (if (not (Variables|Default|GetLoopBroke))
    (return)))