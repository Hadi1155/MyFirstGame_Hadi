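; BP_BaseCollectible is a base pickup actor that bobs vertically and is collected when BP_Eva overlaps its sphere.
; Tick adds a clamped sine offset to its world Z position.
; Overlap calls OnPlayerOverlap, which checks CanBePickedUp (always true here) before OnPickUp plays an optional sound and destroys the actor.
; The construction script creates a dynamic material instance tinted by the Color variable.
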(event OnComponentBeginOverlap(SphereCollision)
  (params (OverlappedComponent :type Primitive%20Component%20Object%20Reference) (OtherActor :type Actor%20Object%20Reference) (OtherComp :type Primitive%20Component%20Object%20Reference) (OtherBodyIndex :type Integer) (bFromSweep :type Boolean) (SweepResult :type Hit%20Result%20Structure%20%28by%20ref%29))
  (bind _asbp_eva (Utilities|Casting|CastToBP_Eva OtherActor))
  (CallFunction|OnPlayerOverlap _asbp_eva))

(event Custom|OnPlayerOverlap
  (params (Character :type BP%20Eva%20Object%20Reference))
  (bind _canbepickedup_ (CallFunction|CanbePickedUp? Character))
  (if _canbepickedup_
    (CallFunction|OnPickUp Character)))

(event Custom|OnPickUp
  (params (Character :type BP%20Eva%20Object%20Reference))
  (bind _sound (Variables|Default|GetSound)
    (:then
      (Audio|PlaySoundatLocation _sound (Transformation|GetWorldLocation (Variables|Default|GetMesh)) "0, 0, 0" 1.0 1.0 0.0 0 0 0 0))
    (:else
      _))
  (Actor|DestroyActor))

(event EventBeginPlay)

(event Collision|EventActorBeginOverlap
  (params (OtherActor :type Actor%20Object%20Reference)))

(event EventTick
  (params (DeltaSeconds :type Float%20%28single-precision%29))
  (bind _output_get (Variables|Default|SetBobbingRange (+ DeltaSeconds (Variables|Default|GetBobbingRange))))
  (Transformation|AddActorWorldOffset (Math|Vector|MakeVector 0.0 0.0 (Math|Float|Clamp(Float) (Math|Trig|Sin(Radians) (* _output_get (Variables|Default|GetSineSpeed))) -0.2 0.2))))

(fn ConstructionScript
  (bind _returnvalue (Rendering|Material|CreateDynamicMaterialInstance (Variables|Default|GetMesh) 0 "/Game/Focus/Assets/Collectible_Base/M_Collectible_Inst.M_Collectible_Inst" "None" :!class /Script/Engine.PrimitiveComponent))
  (bind _output_get (Variables|Default|SetMaterial _returnvalue))
  (Rendering|Material|SetVectorParameterValue _output_get "Color" (Variables|Default|GetColor) :!class /Script/Engine.MaterialInstanceDynamic))

(fn CanbePickedUp?
  (params (Character :type BP%20Eva%20Object%20Reference))
  (return true))