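; BP_AmmunitionDrops is a collectible ammo drop that adds AmmoToAdd to the picking character's AmmoOwned.
; It extends a parent pickup class, overriding OnPickUp to cap the total at MaxCarriedAmmo before calling the parent logic.
; CanBePickedUp calls the parent but ignores its result, allowing pickup only when the full amount fits within that cap.
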(event EventOnPickUp
  (params (Character :type BP%20Eva%20Object%20Reference))
  (bind _maxcarriedammo (Variables|/Game/Focus/Blueprint/Character/BP_Eva.BP_Eva_C|GetMaxCarriedAmmo Character))
  (if (> (+ (Variables|/Game/Focus/Blueprint/Character/BP_Eva.BP_Eva_C|GetAmmoOwned Character) (Variables|Default|GetAmmoToAdd)) _maxcarriedammo)
    (Variables|/Game/Focus/Blueprint/Character/BP_Eva.BP_Eva_C|SetAmmoOwned Character _maxcarriedammo)
    (else
      (Variables|/Game/Focus/Blueprint/Character/BP_Eva.BP_Eva_C|SetAmmoOwned Character (+ (Variables|/Game/Focus/Blueprint/Character/BP_Eva.BP_Eva_C|GetAmmoOwned Character) (Variables|Default|GetAmmoToAdd)))))
  (|CallParentFunction 0))

(fn ConstructionScript
  (|CallParentFunction))

(fn CanbePickedUp?
  (params (Character :type BP%20Eva%20Object%20Reference))
  (|CallParentFunction Character)
  (if (<= (+ (Variables|/Game/Focus/Blueprint/Character/BP_Eva.BP_Eva_C|GetAmmoOwned Character) (Variables|Default|GetAmmoToAdd)) (Variables|/Game/Focus/Blueprint/Character/BP_Eva.BP_Eva_C|GetMaxCarriedAmmo Character))
    (return true)
    (else
      (return false))))