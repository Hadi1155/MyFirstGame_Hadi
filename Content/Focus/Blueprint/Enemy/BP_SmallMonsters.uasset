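; BP_SmallMonsters is a small enemy character that attacks by leaping at a target character.
; Its Attack event waits out a jump cooldown, turns to face the target, then launches forward with an upward boost.
; Its capsule applies a small fixed amount of damage to BP_Eva on overlap, whether or not an attack is in progress.
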(event OnComponentBeginOverlap(CapsuleComponent)
  (params (OverlappedComponent :type Primitive%20Component%20Object%20Reference) (OtherActor :type Actor%20Object%20Reference) (OtherComp :type Primitive%20Component%20Object%20Reference) (OtherBodyIndex :type Integer) (bFromSweep :type Boolean) (SweepResult :type Hit%20Result%20Structure%20%28by%20ref%29))
  (bind _asbp_eva (Utilities|Casting|CastToBP_Eva OtherActor))
  (Game|Damage|ApplyDamage _asbp_eva 3.0 0 0))

(event EventAttack
  (params (Character :type BP%20Eva%20Object%20Reference))
  (bind _returnvalue (Transformation|GetActorRotation))
  (bind _returnvalue_2 (Transformation|GetActorLocation))
  (bind _returnvalue_3 (Transformation|GetActorLocation Character))
  (bind _returnvalue_4 (Math|Conversions|ToTransform(Vector) _returnvalue_2))
  (bind _returnvalue_5 (Math|Vector|GetForwardVector _returnvalue))
  (bind _returnvalue_6 (Math|Rotator|FindRelativeLookatRotation _returnvalue_4 _returnvalue_3))
  (bind _returnvalue_7 (* _returnvalue_5 5e+02))
  (Utilities|FlowControl|Delay (Variables|Default|GetJumpCooldown))
  (Transformation|SetActorRotation (Math|Rotator|MakeRotator (.roll _returnvalue_6) (.pitch _returnvalue_6) (.yaw _returnvalue_6)))
  (Character|LaunchCharacter (Math|Vector|MakeVector (.x _returnvalue_7) (.y _returnvalue_7) (+ (.z _returnvalue_7) 5e+02)) false false))

(fn ConstructionScript
  (|CallParentFunction))