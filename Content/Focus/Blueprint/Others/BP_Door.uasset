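; BP_Door is a locked, interactable door that swings open when the interacting character has a key.
; IsInteractable consumes one key and plays an unlock sound, or plays a locked sound and refuses.
; OnInteract plays an opening sound and runs a timeline that lerps the mesh yaw to swing it open.
; Unlocked is only reset on BeginPlay and never checked, and all sounds play at world origin.
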(event EventBeginPlay
  (Variables|Default|SetUnlocked false))

(event Collision|EventActorBeginOverlap
  (params (OtherActor :type Actor%20Object%20Reference)))

(event EventTick
  (params (DeltaSeconds :type Float%20%28single-precision%29)))

(event EventOnInteract
  (params (Character :type BP%20Eva%20Object%20Reference))
  (Audio|PlaySoundatLocation "/Game/Focus/Assets/Audios/Interactables/SC_DoorOpening.SC_DoorOpening" "0, 0, 0" "0, 0, 0" 1.0 1.0 0.0 0 0 0 0)
  (bind _newtrack_0 (Timeline|DoorOpenTimeline PlayFromStart)
    (:Update
      (Transformation|SetRelativeRotation (Variables|Default|GetMesh) (Math|Rotator|MakeRotator 0.0 0.0 (Math|Float|Lerp 0.0 -1.2e+02 _newtrack_0)) false false))))

(fn ConstructionScript)

(fn IsInteractable?
  (params (Character :type BP%20Eva%20Object%20Reference))
  (if (> (Variables|/Game/Focus/Blueprint/Character/BP_Eva.BP_Eva_C|GetKeyOwned Character) 0)
    (Variables|/Game/Focus/Blueprint/Character/BP_Eva.BP_Eva_C|SetKeyOwned Character (- (Variables|/Game/Focus/Blueprint/Character/BP_Eva.BP_Eva_C|GetKeyOwned Character) 1))
    (Audio|PlaySoundatLocation "/Game/Focus/Assets/Audios/Interactables/unlock-the-door-2-99745__mp3cut_net_.unlock-the-door-2-99745__mp3cut_net_" "0, 0, 0" "0, 0, 0" 1.0 1.0 0.0 0 0 0 0)
    (return true)
    (else
      (Audio|PlaySoundatLocation "/Game/Focus/Assets/Audios/Interactables/SC_LockedDoor.SC_LockedDoor" "0, 0, 0" "0, 0, 0" 1.0 1.0 0.0 0 0 0 0)
      (return false))))

(fn OnDetected
  (return ""))